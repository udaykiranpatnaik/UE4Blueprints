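; BP_SponsorV3 is a sponsor actor for placing patterned static mesh instances along a referenced actor's spline.
; Helpers build transforms at spline points or spaced distances with a lateral offset, and create one HISM component per mesh.
; Pattern values index both the component and transform arrays when adding instances.
; The construction script only caches the spline; instance and pattern generation calls are disconnected, and transform generation is never called here.
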(fn `Generate Instances`
  (params (PatternArray :type "Array of Integer") (Transforms :type "Array of Transform Structure") (StaticMeshList :type "Array of StaticMesh Object Reference"))
  (locals (InstanceComponentList :type "Array of HierarchicalInstancedStaticMeshComponent Object Reference") (`Current Static Mesh` :type "StaticMesh Object Reference") (CurrentInstanceComponent :type "HierarchicalInstancedStaticMeshComponent Object Reference") (Pattern :type "Array of Integer") (InstancePositions :type "Array of Transform Structure"))
  (set `local.Pattern` PatternArray)
  (set `local.InstancePositions` Transforms)
  (`KismetArrayLibrary.Array_Clear` (`local.InstanceComponentList`))
  (for _array_element StaticMeshList
    (set `local.Current Static Mesh` _array_element)
    (bind _returnvalue (`AddComponent|NODE_AddHierarchicalInstancedStaticMeshComponent-1`))
    (bind _output_get (set `local.CurrentInstanceComponent` _returnvalue))
    (`StaticMeshComponent.SetStaticMesh` _output_get (`local.Current Static Mesh`))
    (`KismetArrayLibrary.Array_AddUnique` (`local.InstanceComponentList`) (`local.CurrentInstanceComponent`)))
  (for _array_element_2 (`local.Pattern`)
    (`InstancedStaticMeshComponent.AddInstance` (`|GetArrayItem` (`local.InstanceComponentList`) _array_element_2) (`|GetArrayItem` (`local.InstancePositions`) _array_element_2))))

(fn `Generate Pattern Array`
  (bind ((`NumInstances_28_C40B09A8401F58E83A33A5B1A3DE2307` _numinstances) (`Pattern_21_A20C131B40B96D95C5C34D914F615F6E` _pattern)) (break `/Game/Blueprints/SponsorsV3/Struct_DistributionSettings` (`self.Settings`)))
  (`KismetArrayLibrary.Array_Resize` (`.PatternArray_9_AA40C0254A95482746ED1D94CE5FA0E4` (break `/Game/Blueprints/SponsorsV3/Struct_PatternSettings` _pattern)) _numinstances))

(fn `Set Spline Generation`
  (params (`Num Instance` :type Integer) (Gap :type "Float (double-precision)") (`Lateral Offset` :type "Float (double-precision)"))
  (returns (Positions :type "Array of Transform Structure"))
  (locals (Transforms :type "Array of Transform Structure") (Count :type Integer) (Distance :type "Float (double-precision)") (Offset :type "Float (double-precision)" :default 0.0))
  (set `local.Count` `Num Instance`)
  (set `local.Offset` `Lateral Offset`)
  (`KismetArrayLibrary.Array_Clear` (`local.Transforms`))
  (switch `/Game/Blueprints/SponsorsV3/Enum_SplineGenerationTypes` (`self.GenerationType`)
    (:`NewEnumerator0`
      ;[1 1 1] Spline Points
      (for _index (range (`SplineComponent.GetNumberOfSplinePoints` (`self.SplineComponent`)))
        (`KismetArrayLibrary.Array_AddUnique` (`local.Transforms`) (`SplineComponent.GetTransformAtSplinePoint` (`self.SplineComponent`) _index "Local" false))))
    (:`NewEnumerator1`
      (for _index_2 (range (`local.Count`))
        (set `local.Distance` (* _index_2 Gap))
        (`KismetArrayLibrary.Array_AddUnique` (`local.Transforms`) (`KismetMathLibrary.MakeTransform` (+ (`SplineComponent.GetLocationAtDistanceAlongSpline` (`self.SplineComponent`) (`local.Distance`) "Local") (`KismetMathLibrary.MakeVector` (.x (`SplineComponent.GetRightVectorAtDistanceAlongSpline` (`self.SplineComponent`) (`local.Distance`) "Local")) (* (.y (`SplineComponent.GetRightVectorAtDistanceAlongSpline` (`self.SplineComponent`) (`local.Distance`) "Local")) (`local.Offset`)) (.z (`SplineComponent.GetRightVectorAtDistanceAlongSpline` (`self.SplineComponent`) (`local.Distance`) "Local")))) (`SplineComponent.GetRotationAtDistanceAlongSpline` (`self.SplineComponent`) (`local.Distance`) "Local"))))))
  (return (`local.Transforms`)))

(fn `Set Spline Reference`
  (bind _spline_actor_reference (`self.Spline Actor Reference`))
  (`/Engine/EditorBlueprintResources/StandardMacros.IsValid` _spline_actor_reference
    (:`Is Valid`
      (set `self.SplineComponent` (`self.GetComponentByClass` _spline_actor_reference "/Script/Engine.SplineComponent")))))

(fn `UserConstructionScript`
  (`self.Set Spline Reference`))