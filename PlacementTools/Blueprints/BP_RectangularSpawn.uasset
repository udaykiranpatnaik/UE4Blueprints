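; Placement tool that scatters random meshes as instanced static meshes across a rectangle, with a scaled preview box.
; The construction script reads size, count and seed from axis-locked vector locators, then creates one instance component per mesh entry.
; A seeded stream, optionally location-derived, picks mesh, transform and position, clumped by Full, Edge or Corner mode.
; Optional projection traces along local down, keeping only hits and optionally aligning to the surface.
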(fn `UserConstructionScript`
  (bind _box_x (`self.Box_X`))
  (bind _previewmesh (`self.PreviewMesh`))
  (bind _instances (`self.Instances`))
  (bind _stream (`self.Stream`))
  (bind (_box_x_2 _box_y) (`KismetMathLibrary.BreakVector` (`self.Box`)))
  (bind (_numberofmeshes_x _numberofmeshes_y) (`KismetMathLibrary.BreakVector` (`self.NumberOfMeshes`)))
  (bind (_seed_x _seed_y _seed_z) (`KismetMathLibrary.BreakVector` (`self.Seed`)))
  (bind _box_y_2 (`self.Box_Y`))
  (bind _randomrotation (`self.RandomRotation`))
  (bind (_mesh _rotation_min _rotation_max _scale_min _scale_max _uniformscale) (break `/Game/PlacementTools/Data/Struct_RandomStaticMesh` (`self.CurrentMesh`)))
  (bind _returnvalue (`KismetMathLibrary.RandomFloatInRangeFromStream` 0.0 (`self.Box_Y`) (`self.Stream`)))
  (bind _returnvalue_2 (`KismetMathLibrary.RandomFloatInRangeFromStream` 0.0 (`self.ClumpFactor`) (`self.Stream`)))
  (bind _returnvalue_3 (* (`self.EdgeFactor`) -1.0))
  (bind _returnvalue_4 (`KismetMathLibrary.RandomFloatInRangeFromStream` (.x _scale_min) (.x _scale_max) _stream))
  (bind _returnvalue_5 (+ (`KismetMathLibrary.GreaterGreater_VectorRotator` (`self.RandomLocation`) (`self.K2_GetActorRotation`)) (`self.K2_GetActorLocation`)))
  ;[1 1 1] Update
  (if (`self.Update`)
    _
    (else
      _))
  (set `self.Update` false)
  ;[1 1 1] Get Values from Locators
  (set `self.Box` (`KismetMathLibrary.MakeVector` _box_x_2 _box_y))
  (set `self.Box_X` _box_x_2)
  (set `self.Box_Y` _box_y)
  (set `self.NumberOfMeshes` (`KismetMathLibrary.MakeVector` 0.0 _numberofmeshes_y))
  (set `self.NumberOfMeshes_Value` (`KismetMathLibrary.FTrunc` _numberofmeshes_y))
  (set `self.Seed` (`KismetMathLibrary.MakeVector` 0.0 0.0 _seed_z))
  (set `self.Seed_Value` (`KismetMathLibrary.FTrunc` _seed_z))
  ;[1 1 1] Make Random Seed
  (set `self.Stream` (`KismetMathLibrary.MakeRandomStream` (select `bool` (`self.LocationSeeded`) :`false` (`self.Seed_Value`) :`true` (`KismetMathLibrary.FTrunc` (+ (.x (`self.K2_GetActorLocation`)) (.y (`self.K2_GetActorLocation`)) (.z (`self.K2_GetActorLocation`)))))))
  ;[1 1 1] Set Preview Box
  (`SceneComponent.SetRelativeScale3D` _previewmesh (`KismetMathLibrary.MakeVector` (/ _box_x 50.0) (/ _box_y_2 50.0) 0.01))
  (`SceneComponent.K2_SetRelativeLocation` _previewmesh (`KismetMathLibrary.MakeVector` (/ _box_x 2.0) (/ _box_y_2 2.0)) false false)
  ;[1 1 1] Create Instance Static Meshes
  (for _array_element (`self.Meshes`)
    (bind _returnvalue_6 (`AddComponent|NODE_AddInstancedStaticMeshComponent-1`))
    (bind (_mesh_2 _rotation_min_2 _rotation_max_2 _scale_min_2 _scale_max_2 _uniformscale_2 _castshadow) (break `/Game/PlacementTools/Data/Struct_RandomStaticMesh` _array_element))
    (`StaticMeshComponent.SetStaticMesh` _returnvalue_6 _mesh_2)
    (`PrimitiveComponent.SetCastShadow` _returnvalue_6 _castshadow))
  (set `self.Instances` (`self.K2_GetComponentsByClass` "/Script/Engine.InstancedStaticMeshComponent"))
  ;[1 1 1] Spawn Instances
  (for _ (range (`self.NumberOfMeshes_Value`))
    (bind _output_get (set `self.CurrentMeshIndex` (`KismetMathLibrary.RandomIntegerInRangeFromStream` 0 (- (`KismetArrayLibrary.Array_Length` _instances) 1) (`self.Stream`))))
    (set `self.CurrentMesh` (`|GetArrayItem` (`self.Meshes`) _output_get))
    (set `self.CurrentInstance` (`|GetArrayItem` _instances _output_get))
    (set `self.RandomLocation` (select `/Game/PlacementTools/Data/Enum_ShapeType` (`self.Type`) :`NewEnumerator0` (`KismetMathLibrary.VLerp` (`KismetMathLibrary.MakeVector` (`KismetMathLibrary.RandomFloatInRangeFromStream` 0.0 (`self.Box_X`) (`self.Stream`)) (`KismetMathLibrary.RandomFloatInRangeFromStream` 0.0 (`self.Box_Y`) (`self.Stream`))) (`KismetMathLibrary.MakeVector` (/ (`self.Box_X`) 2.0) (/ (`self.Box_Y`) 2.0)) (`KismetMathLibrary.RandomFloatInRangeFromStream` 0.0 (`self.ClumpFactor`) (`self.Stream`))) :`NewEnumerator3` (`KismetMathLibrary.VLerp` (`KismetMathLibrary.MakeVector` (`KismetMathLibrary.FMax` (`KismetMathLibrary.RandomFloatInRangeFromStream` (* (`self.Box_X`) _returnvalue_3) (`self.Box_X`) (`self.Stream`))) _returnvalue) (`KismetMathLibrary.MakeVector` 0.0 _returnvalue) _returnvalue_2) :`NewEnumerator4` (`KismetMathLibrary.VLerp` (`KismetMathLibrary.MakeVector` (`KismetMathLibrary.FMax` (`KismetMathLibrary.RandomFloatInRangeFromStream` (* (`self.Box_X`) _returnvalue_3) (`self.Box_X`) (`self.Stream`))) (`KismetMathLibrary.FMax` (`KismetMathLibrary.RandomFloatInRangeFromStream` (* (`self.Box_Y`) _returnvalue_3) (`self.Box_Y`) (`self.Stream`)))) (0.0 0.0 0.0) _returnvalue_2)))
    (set `self.RandomScale` (* (select `bool` _uniformscale :`false` (`KismetMathLibrary.MakeVector` _returnvalue_4 (`KismetMathLibrary.RandomFloatInRangeFromStream` (.y _scale_min) (.y _scale_max) _stream) (`KismetMathLibrary.RandomFloatInRangeFromStream` (.z _scale_min) (.z _scale_max) _stream)) :`true` (`KismetMathLibrary.MakeVector` _returnvalue_4 _returnvalue_4 _returnvalue_4)) (`self.GlobalScale`)))
    (set `self.RandomRotation` (`KismetMathLibrary.MakeRotator` (`KismetMathLibrary.RandomFloatInRangeFromStream` (.roll _rotation_min) (.roll _rotation_max) _stream) (`KismetMathLibrary.RandomFloatInRangeFromStream` (.pitch _rotation_min) (.pitch _rotation_max) _stream) (`KismetMathLibrary.RandomFloatInRangeFromStream` (.yaw _rotation_min) (.yaw _rotation_max) _stream)))
    (if (`self.Project`)
      (bind (_outhit _returnvalue_7) (`KismetSystemLibrary.LineTraceSingle` _returnvalue_5 (- _returnvalue_5 (`KismetMathLibrary.GreaterGreater_VectorRotator` (`KismetMathLibrary.MakeVector` 0.0 0.0 (`self.ProjectionDistance`)) (`self.K2_GetActorRotation`))) "TraceTypeQuery1"))
      (if _returnvalue_7
        (bind (_bblockinghit _binitialoverlap _time _distance _location _impactpoint _normal _impactnormal) (`GameplayStatics.BreakHitResult` _outhit))
        (`InstancedStaticMeshComponent.AddInstance` (`self.CurrentInstance`) (`KismetMathLibrary.MakeTransform` (`KismetMathLibrary.InverseTransformLocation` (`self.GetTransform`) _impactpoint) (select `bool` (`self.AlignToSurface`) :`false` _randomrotation :`true` (`KismetMathLibrary.ComposeRotators` _randomrotation (`KismetMathLibrary.ComposeRotators` (`KismetMathLibrary.Conv_VectorToRotator` _impactnormal) (`KismetMathLibrary.NegateRotator` (`self.K2_GetActorRotation`))))) (`self.RandomScale`))))
      (else
        (`InstancedStaticMeshComponent.AddInstance` (`self.CurrentInstance`) (`KismetMathLibrary.MakeTransform` (`self.RandomLocation`) (`self.RandomRotation`) (`self.RandomScale`)))))))