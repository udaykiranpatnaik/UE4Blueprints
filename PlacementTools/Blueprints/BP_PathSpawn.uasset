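; Placement tool that scatters random static mesh instances along a spline at construction time.
; Offset, count and seed come from axis-constrained vector locators; a seeded stream drives mesh choice, position, rotation and scale.
; Each mesh entry gets an instanced static mesh component, with sideways offsets shaped by clump, edge-bias and side-swap settings.
; Optional projection line-traces downward, adding an instance only where the trace hits.
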(fn `UserConstructionScript`
  (bind _numberofmeshes_x (`KismetMathLibrary.BreakVector` (`self.NumberOfMeshes`)))
  (bind _spline (`self.Spline`))
  (bind _meshes (`self.Meshes`))
  (bind _stream (`self.Stream`))
  (bind _stream_2 (`self.Stream`))
  (bind _offsetvalue (`self.OffsetValue`))
  (bind (_maxoffset_x _maxoffset_y) (`KismetMathLibrary.BreakVector` (`self.MaxOffset`)))
  (bind (_seed_x _seed_y _seed_z) (`KismetMathLibrary.BreakVector` (`self.Seed`)))
  (bind _returnvalue (`KismetMathLibrary.RandomFloatInRangeFromStream` (* _offsetvalue -1.0) _offsetvalue (`self.Stream`)))
  (bind _returnvalue_2 (* (`SplineComponent.GetSplineLength` _spline) (`KismetMathLibrary.RandomFloatFromStream` _stream_2)))
  (bind _returnvalue_3 (`KismetMathLibrary.RandomIntegerInRangeFromStream` 0 (- (`KismetArrayLibrary.Array_Length` _meshes) 1) _stream_2))
  (bind _output (`|GetArrayItem` (`self.Instances`) _returnvalue_3))
  (bind _output_2 (`|GetArrayItem` _meshes _returnvalue_3))
  (bind _returnvalue_4 (* (`SplineComponent.GetRightVectorAtDistanceAlongSpline` _spline _returnvalue_2 "Local") (`KismetMathLibrary.Lerp` _returnvalue (`KismetMathLibrary.FMax` _returnvalue) (`self.EdgeFactor`))))
  (bind _returnvalue_5 (`KismetMathLibrary.RandomFloatInRangeFromStream` (.x (`.Scale_Min_5_7DA57470436E509301091287FCCD7893` (break `/Game/PlacementTools/Data/Struct_RandomStaticMesh` _output_2))) (.x (`.Scale_Max_7_DD941EF9488F68923EED648C6FF918C5` (break `/Game/PlacementTools/Data/Struct_RandomStaticMesh` _output_2))) _stream))
  (bind _returnvalue_6 (`KismetMathLibrary.MakeRotator` (`KismetMathLibrary.RandomFloatInRangeFromStream` (.roll (`.Rotation_Min_12_2016FD4941A20E2A8135669D7429D84F` (break `/Game/PlacementTools/Data/Struct_RandomStaticMesh` _output_2))) (.roll (`.Rotation_Max_13_BFF80E0D44951C3943C3D3924455AE45` (break `/Game/PlacementTools/Data/Struct_RandomStaticMesh` _output_2))) _stream) (`KismetMathLibrary.RandomFloatInRangeFromStream` (.pitch (`.Rotation_Min_12_2016FD4941A20E2A8135669D7429D84F` (break `/Game/PlacementTools/Data/Struct_RandomStaticMesh` _output_2))) (.pitch (`.Rotation_Max_13_BFF80E0D44951C3943C3D3924455AE45` (break `/Game/PlacementTools/Data/Struct_RandomStaticMesh` _output_2))) _stream) (`KismetMathLibrary.RandomFloatInRangeFromStream` (.yaw (`.Rotation_Min_12_2016FD4941A20E2A8135669D7429D84F` (break `/Game/PlacementTools/Data/Struct_RandomStaticMesh` _output_2))) (.yaw (`.Rotation_Max_13_BFF80E0D44951C3943C3D3924455AE45` (break `/Game/PlacementTools/Data/Struct_RandomStaticMesh` _output_2))) _stream)))
  (bind _returnvalue_7 (select `bool` (`.UniformScale_17_D870ED2543279348E00E229D1ECDF881` (break `/Game/PlacementTools/Data/Struct_RandomStaticMesh` _output_2)) :`false` (`KismetMathLibrary.MakeVector` _returnvalue_5 (`KismetMathLibrary.RandomFloatInRangeFromStream` (.y (`.Scale_Min_5_7DA57470436E509301091287FCCD7893` (break `/Game/PlacementTools/Data/Struct_RandomStaticMesh` _output_2))) (.y (`.Scale_Max_7_DD941EF9488F68923EED648C6FF918C5` (break `/Game/PlacementTools/Data/Struct_RandomStaticMesh` _output_2))) _stream) (`KismetMathLibrary.RandomFloatInRangeFromStream` (.z (`.Scale_Min_5_7DA57470436E509301091287FCCD7893` (break `/Game/PlacementTools/Data/Struct_RandomStaticMesh` _output_2))) (.z (`.Scale_Max_7_DD941EF9488F68923EED648C6FF918C5` (break `/Game/PlacementTools/Data/Struct_RandomStaticMesh` _output_2))) _stream)) :`true` (`KismetMathLibrary.MakeVector` _returnvalue_5 _returnvalue_5 _returnvalue_5)))
  (bind _returnvalue_8 (`KismetMathLibrary.VLerp` (select `bool` (`self.SwapEdges`) :`false` _returnvalue_4 :`true` (* _returnvalue_4 -1.0)) (0.0 0.0 0.0) (`KismetMathLibrary.RandomFloatInRangeFromStream` 0.0 (`self.ClumpFactor`) (`self.Stream`))))
  (bind _returnvalue_9 (+ (`SplineComponent.GetLocationAtDistanceAlongSpline` _spline _returnvalue_2 "World") _returnvalue_8))
  ;[1 1 1] Update
  (if (`self.Update`)
    _
    (else
      _))
  (set `self.Update` false)
  ;[1 1 1] Get Values from Locators
  (set `self.MaxOffset` (`KismetMathLibrary.MakeVector` 0.0 _maxoffset_y))
  (set `self.OffsetValue` _maxoffset_y)
  (set `self.NumberOfMeshes` (`KismetMathLibrary.MakeVector` _numberofmeshes_x))
  (set `self.NumberOfMeshesValue` (`KismetMathLibrary.FTrunc` _numberofmeshes_x))
  (set `self.Seed` (`KismetMathLibrary.MakeVector` 0.0 0.0 _seed_z))
  (set `self.SeedValue` (`KismetMathLibrary.FTrunc` _seed_z))
  ;[1 1 1] Make Stream
  (set `self.Stream` (`KismetMathLibrary.MakeRandomStream` (`self.SeedValue`)))
  ;[1 1 1] Create Static Mesh Instances
  (for _array_element (`self.Meshes`)
    (bind _returnvalue_10 (`AddComponent|NODE_AddInstancedStaticMeshComponent-0`))
    (bind (_mesh _rotation_min _rotation_max _scale_min _scale_max _uniformscale _castshadow) (break `/Game/PlacementTools/Data/Struct_RandomStaticMesh` _array_element))
    (`StaticMeshComponent.SetStaticMesh` _returnvalue_10 _mesh)
    (`PrimitiveComponent.SetCastShadow` _returnvalue_10 _castshadow))
  (set `self.Instances` (`self.K2_GetComponentsByClass` "/Script/Engine.InstancedStaticMeshComponent"))
  ;[1 1 1] Add Mesh Instances Along Spline
  (for _ (range (`self.NumberOfMeshesValue`))
    (if (`self.Project`)
      (bind (_outhit _returnvalue_11) (`KismetSystemLibrary.LineTraceSingle` _returnvalue_9 (+ _returnvalue_9 (* (0.0 0.0 -1.0) (`self.ProjectionDistance`))) "TraceTypeQuery1"))
      (if _returnvalue_11
        (`InstancedStaticMeshComponent.AddInstance` _output (`KismetMathLibrary.MakeTransform` (- (`.Location` (`GameplayStatics.BreakHitResult` _outhit)) (`self.K2_GetActorLocation`)) _returnvalue_6 _returnvalue_7)))
      (else
        (`InstancedStaticMeshComponent.AddInstance` _output (`KismetMathLibrary.MakeTransform` (+ (`SplineComponent.GetLocationAtDistanceAlongSpline` _spline _returnvalue_2 "Local") _returnvalue_8) _returnvalue_6 _returnvalue_7))))))