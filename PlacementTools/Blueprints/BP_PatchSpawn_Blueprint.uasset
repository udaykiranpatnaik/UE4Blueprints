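; Placement tool that scatters random Blueprints as child actors inside a spline-outlined patch at construction.
; Seeded random points, pulled centerward by ClumpFactor, must pass per-edge cross-product tests, so outlines must be convex and consistently wound; attempts are capped.
; Count and seed come from locator vectors, or seed from actor location; each entry randomizes scale and rotation.
; Optional projection traces down, optionally aligning to surfaces, and defers spawning until all traces finish.
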(fn `UserConstructionScript`
  (bind _spline (`self.Spline`))
  (bind (_testlocation_x _testlocation_y) (`KismetMathLibrary.BreakVector` (`self.TestLocation`)))
  (bind _stream (`self.Stream`))
  (bind _stream_2 (`self.Stream`))
  (bind _blueprints (`self.Blueprints`))
  (bind (_numberofmeshes_x _numberofmeshes_y) (`KismetMathLibrary.BreakVector` (`self.NumberOfMeshes`)))
  (bind (_seed_x _seed_y _seed_z) (`KismetMathLibrary.BreakVector` (`self.Seed`)))
  (bind (_testlocation_x_2 _testlocation_y_2) (`KismetMathLibrary.BreakVector` (`self.TestLocation`)))
  (bind _randomrotation (`self.RandomRotation`))
  (bind _spline_2 (`self.Spline`))
  (bind _splinepoints (`self.SplinePoints`))
  (bind (_blueprint _rotation_min _rotation_max _scale_min _scale_max _uniformscale) (break `/Game/PlacementTools/Data/Struct_RandomBlueprint` (`self.CurrentBlueprint`)))
  (bind _output_blueprint (break `/Game/PlacementTools/Data/Struct_RandomBlueprint` (`|GetArrayItem` (`self.Blueprints`) (`self.CurrentMeshIndex`))))
  (bind _returnvalue (`KismetMathLibrary.RandomFloatInRangeFromStream` 0.0 (* (`KismetMathLibrary.GetPI`) 2.0) _stream))
  (bind _returnvalue_2 (`KismetMathLibrary.Sqrt` (`KismetMathLibrary.RandomFloatFromStream` _stream)))
  (bind _returnvalue_3 (- (`KismetArrayLibrary.Array_Length` _splinepoints) 1))
  (bind _returnvalue_4 (`KismetMathLibrary.RandomFloatInRangeFromStream` (.x _scale_min) (.x _scale_max) _stream_2))
  (bind _returnvalue_5 (+ (`KismetMathLibrary.GreaterGreater_VectorRotator` (`self.RandomLocation`) (`self.K2_GetActorRotation`)) (`self.K2_GetActorLocation`)))
  ;[1 1 1] Update
  (if (`self.Update`)
    _
    (else
      _))
  (set `self.Update` false)
  ;[1 1 1] Get Values from Locators
  (set `self.NumberOfMeshes` (`KismetMathLibrary.MakeVector` 0.0 _numberofmeshes_y))
  (set `self.NumberOfMeshes_Value` (`KismetMathLibrary.FTrunc` _numberofmeshes_y))
  (set `self.Seed` (`KismetMathLibrary.MakeVector` 0.0 0.0 _seed_z))
  (set `self.Seed_Value` (`KismetMathLibrary.FTrunc` _seed_z))
  ;[1 1 1] Make Random Seed
  (set `self.Stream` (`KismetMathLibrary.MakeRandomStream` (select `bool` (`self.LocationSeeded`) :`false` (`self.Seed_Value`) :`true` (`KismetMathLibrary.FTrunc` (+ (.x (`self.K2_GetActorLocation`)) (.y (`self.K2_GetActorLocation`)) (.z (`self.K2_GetActorLocation`)))))))
  ;[1 1 1] Get Spline Data
  (set `self.Radius` 0.0)
  (`KismetArrayLibrary.Array_Clear` (`self.SplinePoints`))
  (for _index (range (`SplineComponent.GetNumberOfSplinePoints` _spline_2))
    (`SplineComponent.SetSplinePointType` _spline_2 _index "Linear" true)
    (bind _returnvalue_6 (+ (`SplineComponent.GetLocationAtSplinePoint` _spline _index "Local") (`SceneComponent.RelativeLocation` _spline)))
    (`KismetArrayLibrary.Array_Add` (`self.SplinePoints`) (`KismetMathLibrary.MakeVector` (.x _returnvalue_6) (.y _returnvalue_6)))
    (bind _returnvalue_7 (`KismetMathLibrary.Sqrt` (`KismetMathLibrary.VSizeSquared` _returnvalue_6)))
    (if (> _returnvalue_7 (`self.Radius`))
      (set `self.Radius` _returnvalue_7)))
  ;[1 1 1] Spawn Instances
  (set `self.CurrentMeshValue` 0)
  (set `self.FailSafe` 0)
  (while (and (< (`self.CurrentMeshValue`) (`self.NumberOfMeshes_Value`)) (< (`self.FailSafe`) (* (`self.NumberOfMeshes_Value`) 2)))
    (`/Engine/EditorBlueprintResources/StandardMacros.IncrementInt` (`self.FailSafe`)
      (:`  `
        ;;[1 1 1] Check Test Point against each Spline Edge
        (set `self.TestFailed` false)
        (set `self.TestLocation` (`KismetMathLibrary.VLerp` (* (`KismetMathLibrary.MakeVector` (* _returnvalue_2 (`KismetMathLibrary.Cos` _returnvalue)) (* _returnvalue_2 (`KismetMathLibrary.Sin` _returnvalue))) (`self.Radius`)) (0.0 0.0 0.0) (`KismetMathLibrary.RandomFloatInRangeFromStream` 0.0 (`self.ClumpFactor`) (`self.Stream`))))
        (for _index_2 (range (+ _returnvalue_3 1))
          (if (== _index_2 _returnvalue_3)
            (bind (_output_x _output_y) (`KismetMathLibrary.BreakVector` (`|GetArrayItem` _splinepoints _index_2)))
            (if (< (- (* (- (.x (`|GetArrayItem` _splinepoints)) _output_x) (- _testlocation_y _output_y)) (* (- (.y (`|GetArrayItem` _splinepoints)) _output_y) (- _testlocation_x _output_x))) 0.0)
              (set `self.TestFailed` true :!label _label)
              (break))
            (else
              (bind (_output_x_2 _output_y_2) (`KismetMathLibrary.BreakVector` (`|GetArrayItem` _splinepoints _index_2)))
              (if (< (- (* (- (.x (`|GetArrayItem` _splinepoints (+ _index_2 1))) _output_x_2) (- _testlocation_y_2 _output_y_2)) (* (- (.y (`|GetArrayItem` _splinepoints (+ _index_2 1))) _output_y_2) (- _testlocation_x_2 _output_x_2))) 0.0)
                (goto _label)))))
        (if (not (`self.TestFailed`))
          (`/Engine/EditorBlueprintResources/StandardMacros.IncrementInt` (`self.CurrentMeshValue`)
            (:`  `
              (bind _output_get (set `self.CurrentMeshIndex` (`KismetMathLibrary.RandomIntegerInRangeFromStream` 0 (- (`KismetArrayLibrary.Array_Length` _blueprints) 1) (`self.Stream`))))
              (set `self.CurrentBlueprint` (`|GetArrayItem` _blueprints _output_get))
              (set `self.RandomLocation` (`self.TestLocation`))
              (set `self.RandomScale` (* (select `bool` _uniformscale :`false` (`KismetMathLibrary.MakeVector` _returnvalue_4 (`KismetMathLibrary.RandomFloatInRangeFromStream` (.y _scale_min) (.y _scale_max) _stream_2) (`KismetMathLibrary.RandomFloatInRangeFromStream` (.z _scale_min) (.z _scale_max) _stream_2)) :`true` (`KismetMathLibrary.MakeVector` _returnvalue_4 _returnvalue_4 _returnvalue_4)) (`self.GlobalScale`)))
              (set `self.RandomRotation` (`KismetMathLibrary.MakeRotator` (`KismetMathLibrary.RandomFloatInRangeFromStream` (.roll _rotation_min) (.roll _rotation_max) _stream_2) (`KismetMathLibrary.RandomFloatInRangeFromStream` (.pitch _rotation_min) (.pitch _rotation_max) _stream_2) (`KismetMathLibrary.RandomFloatInRangeFromStream` (.yaw _rotation_min) (.yaw _rotation_max) _stream_2)))
              (if (`self.Project`)
                (bind (_outhit _returnvalue_8) (`KismetSystemLibrary.LineTraceSingle` _returnvalue_5 (- _returnvalue_5 (`KismetMathLibrary.GreaterGreater_VectorRotator` (`KismetMathLibrary.MakeVector` 0.0 0.0 (`self.ProjectionDistance`)) (`self.K2_GetActorRotation`))) "TraceTypeQuery1"))
                (if _returnvalue_8
                  (bind (_bblockinghit _binitialoverlap _time _location _impactpoint _normal _impactnormal) (`GameplayStatics.BreakHitResult` _outhit))
                  (`KismetArrayLibrary.Array_Add` (`self.SpawnTransforms`) (`KismetMathLibrary.MakeTransform` (`KismetMathLibrary.InverseTransformLocation` (`self.GetTransform`) _impactpoint) (select `bool` (`self.AlignToSurface`) :`false` _randomrotation :`true` (`KismetMathLibrary.ComposeRotators` _randomrotation (`KismetMathLibrary.ComposeRotators` (`KismetMathLibrary.Conv_VectorToRotator` _impactnormal) (`KismetMathLibrary.NegateRotator` (`self.K2_GetActorRotation`))))) (`self.RandomScale`)))
                  (`KismetArrayLibrary.Array_Add` (`self.SpawnIndicies`) (`self.CurrentMeshIndex`)))
                (else
                  (bind _returnvalue_9 (`AddComponent|NODE_AddChildActorComponent-0` :`RelativeTransform` (`KismetMathLibrary.MakeTransform` (`self.RandomLocation`) (`self.RandomRotation`) (`self.RandomScale`))))
                  (`ChildActorComponent.SetChildActorClass` _returnvalue_9 _output_blueprint)))))))))
  (for (_array_element _array_index) (`self.SpawnTransforms`)
    (bind _returnvalue_10 (`AddComponent|NODE_AddChildActorComponent-1` :`RelativeTransform` (`KismetMathLibrary.MakeTransform` (.location _array_element) (.rotation _array_element) (.scale _array_element))))
    (bind _output_blueprint_2 (break `/Game/PlacementTools/Data/Struct_RandomBlueprint` (`|GetArrayItem` (`self.Blueprints`) (`|GetArrayItem` (`self.SpawnIndicies`) _array_index))))
    (`ChildActorComponent.SetChildActorClass` _returnvalue_10 _output_blueprint_2)
    (if (`self.AlignToSurface`)
      (`SceneComponent.K2_AddLocalRotation` _returnvalue_10 (struct :`Pitch` -90.0) false false))))