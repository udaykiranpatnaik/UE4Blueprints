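; BP_Randomiser is a placement tool that randomises static mesh actors sharing a chosen tag.
; Numbered events randomise mesh, transform, slot-0 material or visibility, or clear all tags, each rebuilding the target list through BuildMeshArray and emptying it afterwards.
; Location offsets add to current positions, while rotation and scale are replaced.
; UniformScale draws each axis separately from the X range, so scale can still differ per axis.
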(event `1_RandomiseMeshes`
  (bind _meshes (`self.Meshes`))
  ;[1 1 1] Randomise Static Mesh
  (`self.BuildMeshArray`)
  (for _array_element (`self.MeshesToRandomise`)
    (bind _asstatic_mesh_actor (cast `StaticMeshActor` _array_element))
    (`StaticMeshComponent.SetStaticMesh` (`StaticMeshActor.StaticMeshComponent` _asstatic_mesh_actor) (`|GetArrayItem` _meshes (`KismetMathLibrary.RandomIntegerInRange` 0 (- (`KismetArrayLibrary.Array_Length` _meshes) 1)))))
  (`KismetArrayLibrary.Array_Clear` (`self.MeshesToRandomise`)))

(event `2_RandomiseTransform`
  (bind (_offset_min _offset_max _rotation_min _rotation_max _scale_min _scale_max _uniformscale) (break `/Game/PlacementTools/Data/Struct_RandomTransform` (`self.Transform`)))
  (bind _returnvalue (`KismetMathLibrary.RandomFloatInRange` (.x _scale_min) (.x _scale_max)))
  ;[1 1 1] Randomise Transform
  (`self.BuildMeshArray`)
  (for _array_element (`self.MeshesToRandomise`)
    (`self.K2_SetActorTransform` _array_element (`KismetMathLibrary.MakeTransform` (+ (`self.K2_GetActorLocation` _array_element) (`KismetMathLibrary.MakeVector` (`KismetMathLibrary.RandomFloatInRange` (.x _offset_min) (.x _offset_max)) (`KismetMathLibrary.RandomFloatInRange` (.y _offset_min) (.y _offset_max)) (`KismetMathLibrary.RandomFloatInRange` (.z _offset_min) (.z _offset_max)))) (`KismetMathLibrary.MakeRotator` (`KismetMathLibrary.RandomFloatInRange` (.roll _rotation_min) (.roll _rotation_max)) (`KismetMathLibrary.RandomFloatInRange` (.pitch _rotation_min) (.pitch _rotation_max)) (`KismetMathLibrary.RandomFloatInRange` (.yaw _rotation_min) (.yaw _rotation_max))) (select `bool` _uniformscale :`false` (`KismetMathLibrary.MakeVector` _returnvalue (`KismetMathLibrary.RandomFloatInRange` (.y _scale_min) (.y _scale_max)) (`KismetMathLibrary.RandomFloatInRange` (.z _scale_min) (.z _scale_max))) :`true` (`KismetMathLibrary.MakeVector` _returnvalue _returnvalue _returnvalue))) false false))
  (`KismetArrayLibrary.Array_Clear` (`self.MeshesToRandomise`)))

(event `3_RandomiseMaterial`
  (bind _materials (`self.Materials`))
  ;[1 1 1] Random Material
  (`self.BuildMeshArray`)
  (for _array_element (`self.MeshesToRandomise`)
    (bind _asstatic_mesh_actor (cast `StaticMeshActor` _array_element))
    (`PrimitiveComponent.SetMaterial` (`StaticMeshActor.StaticMeshComponent` _asstatic_mesh_actor) 0 (`|GetArrayItem` _materials (`KismetMathLibrary.RandomIntegerInRange` 0 (- (`KismetArrayLibrary.Array_Length` _materials) 1)))))
  (`KismetArrayLibrary.Array_Clear` (`self.MeshesToRandomise`)))

(event `4_RandomiseVisibility`
  ;[1 1 1] Randomise Visibility
  (`self.BuildMeshArray`)
  (for _array_element (`self.MeshesToRandomise`)
    (bind _asstatic_mesh_actor (cast `StaticMeshActor` _array_element))
    (if (> (`KismetMathLibrary.RandomFloat`) (`self.PercentageVisibility`))
      (bind _staticmeshcomponent (`StaticMeshActor.StaticMeshComponent` _asstatic_mesh_actor))
      (`SceneComponent.SetVisibility` _staticmeshcomponent false false)
      (else
        (`SceneComponent.SetVisibility` _staticmeshcomponent true false))))
  (`KismetArrayLibrary.Array_Clear` (`self.MeshesToRandomise`)))

(event `5_ClearTags`
  ;[1 1 1] Clear Tags
  (`self.BuildMeshArray`)
  (for _array_element (`self.MeshesToRandomise`)
    (set `Actor.Tags` (`|MakeArray`) _array_element))
  (`KismetArrayLibrary.Array_Clear` (`self.MeshesToRandomise`)))

(fn `BuildMeshArray`
  (bind _outactors (`GameplayStatics.GetAllActorsWithTag` (`self.TagToRandomise`)))
  (for _array_element _outactors
    (bind _asstatic_mesh_actor (cast `StaticMeshActor` _array_element))
    (`KismetArrayLibrary.Array_Add` (`self.MeshesToRandomise`) _asstatic_mesh_actor)))

(fn `UserConstructionScript`)