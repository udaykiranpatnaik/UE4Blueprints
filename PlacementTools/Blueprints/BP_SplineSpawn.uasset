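; BP_SplineSpawn is a placement tool that populates a spline with meshes in its construction script.
; Each spline point can get an instanced static mesh with randomized rotation and scale.
; Each segment can get a deformed spline mesh component, with meshes picked sequentially or from a seeded random stream.
; Optional downward traces project both kinds onto surfaces below and can align them to hit normals, skipping placements where traces miss.
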(fn `UserConstructionScript`
  (bind _spline (`self.Spline`))
  (bind _tangentmultiplier (`self.TangentMultiplier`))
  (bind _instances (`self.Instances`))
  (bind _stream (`self.Stream`))
  (bind _projectsplinemeshes (`self.ProjectSplineMeshes`))
  (bind _projectsplinemeshes_2 (`self.ProjectSplineMeshes`))
  (bind _splinemeshes (`self.SplineMeshes`))
  (bind _alignpointmeshtosurface (`self.AlignPointMeshToSurface`))
  (bind _splineloopindex (`self.SplineLoopIndex`))
  (bind _spline_2 (`self.Spline`))
  (bind _spline_3 (`self.Spline`))
  (bind _currentsplinemesh (`self.CurrentSplineMesh`))
  (bind _returnvalue (`KismetArrayLibrary.Array_Length` _instances))
  (bind _returnvalue_2 (`KismetArrayLibrary.Array_Length` _splinemeshes))
  (bind (_location _tangent) (`SplineComponent.GetLocationAndTangentAtSplinePoint` _spline_3 _splineloopindex "Local"))
  (bind _returnvalue_3 (* (0.0 0.0 -1.0) (`self.SplineProjectionDistance`)))
  (bind _returnvalue_4 (+ _splineloopindex 1))
  (bind _location_2 (`SplineComponent.GetLocationAndTangentAtSplinePoint` _spline_2 (+ (`self.SplineLoopIndex`) 1) "World"))
  (bind (_location_3 _tangent_2) (`SplineComponent.GetLocationAndTangentAtSplinePoint` _spline_3 _returnvalue_4 "Local"))
  ;[1 1 1] Update
  (if (`self.Update`)
    _
    (else
      _))
  (set `self.Update` false)
  ;[1 1 1] Make Random Stream
  (set `self.Stream` (`KismetMathLibrary.MakeRandomStream` (`self.Seed`)))
  ;[1 1 1] Make Instance Components
  (for (_ _array_index) (`self.PointMeshes`)
    (bind _returnvalue_5 (`AddComponent|NODE_AddInstancedStaticMeshComponent-0`))
    (bind (_output_mesh _output_rotation_min _output_rotation_max _output_scale_min _output_scale_max _output_uniformscale _output_castshadow) (break `/Game/PlacementTools/Data/Struct_RandomStaticMesh` (`|GetArrayItem` (`self.PointMeshes`) _array_index)))
    (`StaticMeshComponent.SetStaticMesh` _returnvalue_5 _output_mesh)
    (`PrimitiveComponent.SetCastShadow` _returnvalue_5 _output_castshadow))
  (set `self.Instances` (`self.K2_GetComponentsByClass` "/Script/Engine.InstancedStaticMeshComponent"))
  ;[1 1 1] Add Spline Point Meshes
  (if (`self.IncludePointMeshes`)
    (for _index (range (`SplineComponent.GetNumberOfSplinePoints` (`self.Spline`)))
      (if (`self.ProjectPointMeshes`)
        (bind _location_4 (`SplineComponent.GetLocationAndTangentAtSplinePoint` _spline _index "World"))
        (bind (_outhit _returnvalue_6) (`KismetSystemLibrary.LineTraceSingle` _location_4 (+ _location_4 (* (0.0 0.0 -1.0) (`self.PointProjectionDistance`))) "TraceTypeQuery1"))
        (if _returnvalue_6
          (bind _returnvalue_7 (select `bool` (`self.SequentialMeshes`) :`false` (`KismetMathLibrary.RandomIntegerInRangeFromStream` 0 (- _returnvalue 1) (`self.Stream`)) :`true` (mod _index _returnvalue)))
          (bind _output (`|GetArrayItem` _instances _returnvalue_7))
          (bind (_bblockinghit _binitialoverlap _time _distance _location_5 _impactpoint _normal) (`GameplayStatics.BreakHitResult` _outhit))
          (bind _output_2 (`|GetArrayItem` (`self.PointMeshes`) _returnvalue_7))
          (bind _returnvalue_8 (`KismetMathLibrary.MakeRotator` (`KismetMathLibrary.RandomFloatInRangeFromStream` (.roll (`.Rotation_Min_12_2016FD4941A20E2A8135669D7429D84F` (break `/Game/PlacementTools/Data/Struct_RandomStaticMesh` _output_2))) (.roll (`.Rotation_Max_13_BFF80E0D44951C3943C3D3924455AE45` (break `/Game/PlacementTools/Data/Struct_RandomStaticMesh` _output_2))) _stream) (`KismetMathLibrary.RandomFloatInRangeFromStream` (.pitch (`.Rotation_Min_12_2016FD4941A20E2A8135669D7429D84F` (break `/Game/PlacementTools/Data/Struct_RandomStaticMesh` _output_2))) (.pitch (`.Rotation_Max_13_BFF80E0D44951C3943C3D3924455AE45` (break `/Game/PlacementTools/Data/Struct_RandomStaticMesh` _output_2))) _stream) (`KismetMathLibrary.RandomFloatInRangeFromStream` (.yaw (`.Rotation_Min_12_2016FD4941A20E2A8135669D7429D84F` (break `/Game/PlacementTools/Data/Struct_RandomStaticMesh` _output_2))) (.yaw (`.Rotation_Max_13_BFF80E0D44951C3943C3D3924455AE45` (break `/Game/PlacementTools/Data/Struct_RandomStaticMesh` _output_2))) _stream)))
          (bind (_location_6 _tangent_3) (`SplineComponent.GetLocationAndTangentAtSplinePoint` _spline _index "Local"))
          (bind _returnvalue_9 (select `bool` (`self.AlignToSpline`) :`false` _returnvalue_8 :`true` (`KismetMathLibrary.ComposeRotators` (`KismetMathLibrary.Conv_VectorToRotator` _tangent_3) _returnvalue_8)))
          (bind _returnvalue_10 (`KismetMathLibrary.RandomFloatInRangeFromStream` (.x (`.Scale_Min_5_7DA57470436E509301091287FCCD7893` (break `/Game/PlacementTools/Data/Struct_RandomStaticMesh` _output_2))) (.x (`.Scale_Max_7_DD941EF9488F68923EED648C6FF918C5` (break `/Game/PlacementTools/Data/Struct_RandomStaticMesh` _output_2))) _stream))
          (bind _returnvalue_11 (select `bool` (`.UniformScale_17_D870ED2543279348E00E229D1ECDF881` (break `/Game/PlacementTools/Data/Struct_RandomStaticMesh` _output_2)) :`false` (`KismetMathLibrary.MakeVector` _returnvalue_10 (`KismetMathLibrary.RandomFloatInRangeFromStream` (.y (`.Scale_Min_5_7DA57470436E509301091287FCCD7893` (break `/Game/PlacementTools/Data/Struct_RandomStaticMesh` _output_2))) (.y (`.Scale_Max_7_DD941EF9488F68923EED648C6FF918C5` (break `/Game/PlacementTools/Data/Struct_RandomStaticMesh` _output_2))) _stream) (`KismetMathLibrary.RandomFloatInRangeFromStream` (.z (`.Scale_Min_5_7DA57470436E509301091287FCCD7893` (break `/Game/PlacementTools/Data/Struct_RandomStaticMesh` _output_2))) (.z (`.Scale_Max_7_DD941EF9488F68923EED648C6FF918C5` (break `/Game/PlacementTools/Data/Struct_RandomStaticMesh` _output_2))) _stream)) :`true` (`KismetMathLibrary.MakeVector` _returnvalue_10 _returnvalue_10 _returnvalue_10)))
          (`InstancedStaticMeshComponent.AddInstance` _output (`KismetMathLibrary.MakeTransform` (- _location_5 (`self.K2_GetActorLocation`)) (select `bool` (and _alignpointmeshtosurface (`self.AlignToSpline`)) :`false` (select `bool` _alignpointmeshtosurface :`false` _returnvalue_9 :`true` (`KismetMathLibrary.ComposeRotators` (`KismetMathLibrary.Conv_VectorToRotator` _normal) _returnvalue_8)) :`true` (`KismetMathLibrary.ComposeRotators` (`KismetMathLibrary.MakeRotFromXZ` _normal _tangent_3) _returnvalue_8)) _returnvalue_11)))
        (else
          (`InstancedStaticMeshComponent.AddInstance` _output (`KismetMathLibrary.MakeTransform` _location_6 _returnvalue_9 _returnvalue_11))))))
  ;[1 1 1] Add Spline Meshes
  (if (`self.IncludeSplineMeshes`)
    (for _index_2 (range (+ (- (`SplineComponent.GetNumberOfSplinePoints` (`self.Spline`)) 2) 1))
      (bind _output_get (set `self.SplineLoopIndex` _index_2))
      (if (`self.ProjectSplineMeshes`)
        (bind _location_7 (`SplineComponent.GetLocationAndTangentAtSplinePoint` _spline_2 _output_get "World"))
        (bind (_outhit_2 _returnvalue_12) (`KismetSystemLibrary.LineTraceSingle` _location_7 (+ _location_7 _returnvalue_3) "TraceTypeQuery1"))
        (bind (_outhit_3 _returnvalue_13) (`KismetSystemLibrary.LineTraceSingle` _location_2 (+ _location_2 _returnvalue_3) "TraceTypeQuery1"))
        (if (and _returnvalue_12 _returnvalue_13)
          (bind _returnvalue_14 (`AddComponent|NODE_AddSplineMeshComponent-0` :!label _label))
          (bind _output_get_2 (set `self.CurrentSplineMesh` _returnvalue_14))
          (bind (_bblockinghit_2 _binitialoverlap_2 _time_2 _distance_2 _location_8 _impactpoint_2 _normal_2) (`GameplayStatics.BreakHitResult` _outhit_2))
          (bind (_bblockinghit_3 _binitialoverlap_3 _time_3 _distance_3 _location_9 _impactpoint_3 _normal_3) (`GameplayStatics.BreakHitResult` _outhit_3))
          (`SplineMeshComponent.SetStartAndEnd` _output_get_2 (select `bool` _projectsplinemeshes :`false` _location :`true` (- _location_8 (`self.K2_GetActorLocation`))) (select `bool` (and _projectsplinemeshes (`self.AlignSplineMeshToSurface`)) :`false` _tangent :`true` (* (* (`KismetMathLibrary.Cross_VectorVector` (`SplineComponent.GetRightVectorAtSplinePoint` _spline_3 _splineloopindex "World") _normal_2) (`KismetMathLibrary.VSize` _tangent)) _tangentmultiplier)) (select `bool` _projectsplinemeshes_2 :`false` _location_3 :`true` (- _location_9 (`self.K2_GetActorLocation`))) (select `bool` (and _projectsplinemeshes_2 (`self.AlignSplineMeshToSurface`)) :`false` _tangent_2 :`true` (* (* (`KismetMathLibrary.Cross_VectorVector` (`SplineComponent.GetRightVectorAtSplinePoint` _spline_3 _returnvalue_4 "World") _normal_3) (`KismetMathLibrary.VSize` _tangent_2)) _tangentmultiplier)) false)
          (bind _output_get_3 (set `self.CurrentIndex` (select `bool` (`self.SequentialSplineMeshes`) :`false` (`KismetMathLibrary.RandomIntegerInRangeFromStream` 0 (- _returnvalue_2 1) (`self.Stream`)) :`true` (mod (`self.SplineLoopIndex`) _returnvalue_2))))
          (bind _output_3 (`|GetArrayItem` _splinemeshes _output_get_3))
          (`StaticMeshComponent.SetStaticMesh` _currentsplinemesh (break `/Game/PlacementTools/Data/Struct_RandomSplineMesh` _output_3))
          (`SplineMeshComponent.SetStartScale` _currentsplinemesh (`KismetMathLibrary.MakeVector2D` (.x (`.StartScale_5_BFD77BC04DEF335AD9D7D09538871AE6` (break `/Game/PlacementTools/Data/Struct_RandomSplineMesh` _output_3))) (.y (`.StartScale_5_BFD77BC04DEF335AD9D7D09538871AE6` (break `/Game/PlacementTools/Data/Struct_RandomSplineMesh` _output_3)))) false)
          (`SplineMeshComponent.SetEndScale` _currentsplinemesh (`KismetMathLibrary.MakeVector2D` (.x (`.EndScale_7_2EDDDB3D41A1AD9E001AF0BCD7F0502D` (break `/Game/PlacementTools/Data/Struct_RandomSplineMesh` _output_3))) (.y (`.EndScale_7_2EDDDB3D41A1AD9E001AF0BCD7F0502D` (break `/Game/PlacementTools/Data/Struct_RandomSplineMesh` _output_3)))) false)
          (`SplineMeshComponent.SetStartRoll` _currentsplinemesh (`KismetMathLibrary.RandomFloatInRangeFromStream` (`.Roll_Min_17_78A9D6E0489A3236C83094B3D3A99436` (break `/Game/PlacementTools/Data/Struct_RandomSplineMesh` _output_3)) (`.Roll_Max_16_32381A5B43167E558443B285FC736EA0` (break `/Game/PlacementTools/Data/Struct_RandomSplineMesh` _output_3)) (`self.Stream`)) false)
          (`SplineMeshComponent.SetEndRoll` _currentsplinemesh (`KismetMathLibrary.RandomFloatInRangeFromStream` 0.0 0.0 (`self.Stream`)) true))
        (else
          (goto _label))))))