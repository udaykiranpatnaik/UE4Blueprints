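; Editor placement tool that scatters random Blueprints from a list as child actors within a full, half or quarter circle.
; The construction script reads radius, count and seed from axis-locked locator vectors and sizes a matching preview mesh.
; A random stream, seeded manually or by location, drives clump/edge-biased positions and per-entry scale and rotation.
; Optional projection traces along local down, spawning only on hits, optionally surface-aligned.
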(fn `UserConstructionScript`
  (bind _blueprints (`self.Blueprints`))
  (bind _stream (`self.Stream`))
  (bind _radius_x (`KismetMathLibrary.BreakVector` (`self.Radius`)))
  (bind (_numberofmeshes_x _numberofmeshes_y) (`KismetMathLibrary.BreakVector` (`self.NumberOfMeshes`)))
  (bind (_seed_x _seed_y _seed_z) (`KismetMathLibrary.BreakVector` (`self.Seed`)))
  (bind _stream_2 (`self.Stream`))
  (bind _randomrotation (`self.RandomRotation`))
  (bind _edgefactor (`self.EdgeFactor`))
  (bind (_blueprint _rotation_min _rotation_max _scale_min _scale_max _uniformscale) (break `/Game/PlacementTools/Data/Struct_RandomBlueprint` (`self.CurrentBP`)))
  (bind _returnvalue (/ (`self.Radius_Value`) 25.0))
  (bind _output_blueprint (break `/Game/PlacementTools/Data/Struct_RandomBlueprint` (`|GetArrayItem` (`self.Blueprints`) (`self.CurrentIndex`))))
  (bind _returnvalue_2 (`KismetMathLibrary.RandomFloatInRangeFromStream` 0.0 (* (`KismetMathLibrary.GetPI`) 2.0) _stream_2))
  (bind _returnvalue_3 (`KismetMathLibrary.Sqrt` (`KismetMathLibrary.RandomFloatFromStream` _stream_2)))
  (bind _returnvalue_4 (`KismetMathLibrary.RandomFloatInRangeFromStream` (.x _scale_min) (.x _scale_max) _stream))
  (bind _returnvalue_5 (+ (`KismetMathLibrary.GreaterGreater_VectorRotator` (`self.RandomLocation`) (`self.K2_GetActorRotation`)) (`self.K2_GetActorLocation`)))
  (bind _returnvalue_6 (`KismetMathLibrary.VLerp` (* (`KismetMathLibrary.MakeVector` (* _returnvalue_3 (`KismetMathLibrary.Cos` _returnvalue_2)) (* _returnvalue_3 (`KismetMathLibrary.Sin` _returnvalue_2))) (`self.Radius_Value`)) (0.0 0.0 0.0) (`KismetMathLibrary.RandomFloatInRangeFromStream` 0.0 (`self.ClumpFactor`) (`self.Stream`))))
  ;[1 1 1] Update
  (if (`self.Update`)
    _
    (else
      _))
  (set `self.Update` false)
  ;[1 1 1] Get Values from Locators
  (set `self.Radius` (`KismetMathLibrary.MakeVector` _radius_x))
  (set `self.Radius_Value` _radius_x)
  (set `self.NumberOfMeshes` (`KismetMathLibrary.MakeVector` 0.0 _numberofmeshes_y))
  (set `self.NumberOfMeshes_Value` (`KismetMathLibrary.FTrunc` _numberofmeshes_y))
  (set `self.Seed` (`KismetMathLibrary.MakeVector` 0.0 0.0 _seed_z))
  (set `self.Seed_Value` (`KismetMathLibrary.FTrunc` _seed_z))
  ;[1 1 1] Make Random Seed
  (set `self.Stream` (`KismetMathLibrary.MakeRandomStream` (select `bool` (`self.LocationSeeded`) :`false` (`self.Seed_Value`) :`true` (`KismetMathLibrary.FTrunc` (+ (.x (`self.K2_GetActorLocation`)) (.y (`self.K2_GetActorLocation`)) (.z (`self.K2_GetActorLocation`)))))))
  ;[1 1 1] Set Preview Cylinder Radius
  (`SceneComponent.SetRelativeScale3D` (`self.PreviewMesh`) (`KismetMathLibrary.MakeVector` _returnvalue _returnvalue 0.01))
  (`StaticMeshComponent.SetStaticMesh` (`self.PreviewMesh`) (select `/Game/PlacementTools/Data/Enum_ShapeType` (`self.Type`) :`NewEnumerator0` "/Game/PlacementTools/Meshes/SM_Cylinder.SM_Cylinder" :`NewEnumerator3` "/Game/PlacementTools/Meshes/SM_HalfCylinder.SM_HalfCylinder" :`NewEnumerator4` "/Game/PlacementTools/Meshes/SM_QuarterCylinder.SM_QuarterCylinder" :!type "StaticMesh Object Reference"))
  ;[1 1 1] Spawn Instances
  (for _ (range (`self.NumberOfMeshes_Value`))
    (bind _output_get (set `self.CurrentIndex` (`KismetMathLibrary.RandomIntegerInRangeFromStream` 0 (- (`KismetArrayLibrary.Array_Length` _blueprints) 1) (`self.Stream`))))
    (set `self.CurrentBP` (`|GetArrayItem` _blueprints _output_get))
    (set `self.RandomLocation` (select `/Game/PlacementTools/Data/Enum_ShapeType` (`self.Type`) :`NewEnumerator0` _returnvalue_6 :`NewEnumerator3` (`KismetMathLibrary.VLerp` (`KismetMathLibrary.MakeVector` (`KismetMathLibrary.Abs` (.x _returnvalue_6)) (.y _returnvalue_6) (.z _returnvalue_6)) (`KismetMathLibrary.MakeVector` (`KismetMathLibrary.FMax` (.x _returnvalue_6)) (.y _returnvalue_6) (.z _returnvalue_6)) _edgefactor) :`NewEnumerator4` (`KismetMathLibrary.VLerp` (`KismetMathLibrary.MakeVector` (`KismetMathLibrary.Abs` (.x _returnvalue_6)) (`KismetMathLibrary.Abs` (.y _returnvalue_6)) (.z _returnvalue_6)) (`KismetMathLibrary.MakeVector` (`KismetMathLibrary.FMax` (.x _returnvalue_6)) (`KismetMathLibrary.FMax` (.y _returnvalue_6)) (.z _returnvalue_6)) _edgefactor)))
    (set `self.RandomScale` (* (select `bool` _uniformscale :`false` (`KismetMathLibrary.MakeVector` _returnvalue_4 (`KismetMathLibrary.RandomFloatInRangeFromStream` (.y _scale_min) (.y _scale_max) _stream) (`KismetMathLibrary.RandomFloatInRangeFromStream` (.z _scale_min) (.z _scale_max) _stream)) :`true` (`KismetMathLibrary.MakeVector` _returnvalue_4 _returnvalue_4 _returnvalue_4)) (`self.GlobalScale`)))
    (set `self.RandomRotation` (`KismetMathLibrary.MakeRotator` (`KismetMathLibrary.RandomFloatInRangeFromStream` (.roll _rotation_min) (.roll _rotation_max) _stream) (`KismetMathLibrary.RandomFloatInRangeFromStream` (.pitch _rotation_min) (.pitch _rotation_max) _stream) (`KismetMathLibrary.RandomFloatInRangeFromStream` (.yaw _rotation_min) (.yaw _rotation_max) _stream)))
    (if (`self.Project`)
      (bind (_outhit _returnvalue_7) (`KismetSystemLibrary.LineTraceSingle` _returnvalue_5 (- _returnvalue_5 (`KismetMathLibrary.GreaterGreater_VectorRotator` (`KismetMathLibrary.MakeVector` 0.0 0.0 (`self.ProjectionDistance`)) (`self.K2_GetActorRotation`))) "TraceTypeQuery1"))
      (if _returnvalue_7
        (bind (_bblockinghit _binitialoverlap _time _location _impactpoint _normal _impactnormal) (`GameplayStatics.BreakHitResult` _outhit))
        (`KismetArrayLibrary.Array_Add` (`self.SpawnTransforms`) (`KismetMathLibrary.MakeTransform` (`KismetMathLibrary.InverseTransformLocation` (`self.GetTransform`) _impactpoint) (select `bool` (`self.AlignToSurface`) :`false` _randomrotation :`true` (`KismetMathLibrary.ComposeRotators` _randomrotation (`KismetMathLibrary.ComposeRotators` (`KismetMathLibrary.Conv_VectorToRotator` _impactnormal) (`KismetMathLibrary.NegateRotator` (`self.K2_GetActorRotation`))))) (`self.RandomScale`)))
        (`KismetArrayLibrary.Array_Add` (`self.SpawnIndicies`) (`self.CurrentIndex`)))
      (else
        (bind _returnvalue_8 (`AddComponent|NODE_AddChildActorComponent-0` :`RelativeTransform` (`KismetMathLibrary.MakeTransform` (`self.RandomLocation`) (`self.RandomRotation`) (`self.RandomScale`))))
        (`ChildActorComponent.SetChildActorClass` _returnvalue_8 _output_blueprint))))
  (for (_array_element _array_index) (`self.SpawnTransforms`)
    (bind _returnvalue_9 (`AddComponent|NODE_AddChildActorComponent-1` :`RelativeTransform` (`KismetMathLibrary.MakeTransform` (.location _array_element) (.rotation _array_element) (.scale _array_element))))
    (bind _output_blueprint_2 (break `/Game/PlacementTools/Data/Struct_RandomBlueprint` (`|GetArrayItem` (`self.Blueprints`) (`|GetArrayItem` (`self.SpawnIndicies`) _array_index))))
    (`ChildActorComponent.SetChildActorClass` _returnvalue_9 _output_blueprint_2)
    (if (`self.AlignToSurface`)
      (`SceneComponent.K2_AddLocalRotation` _returnvalue_9 (struct :`Pitch` -90.0) false false))))