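; B_Banners is a procedural-building banner actor that sets up a simple banner, square banner or flag.
; Its construction script switches on BannerType to pick the skeletal mesh, capping the material variant for square banners and flags.
; A per-type offset plus the variant number indexes one shared Materials array, and the result goes on the mesh's "banner" slot.
; The event graph holds no gameplay logic.
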(fn `UserConstructionScript`
  (bind _type_material_banner (`self.Type Material Banner`))
  (bind _skeletalmesh (`self.SkeletalMesh`))
  (bind _skeletalmesh_2 (`self.SkeletalMesh`))
  ;[0 0.5633 1] Static Mesh Select
  (switch `string` (`|GetEnumeratorNameAsString` (`self.Banner Type`))
    (:`Default`
      (`SkinnedMeshComponent.SetSkinnedAssetAndUpdate` _skeletalmesh_2 "/Game/ProceduralBuildings/Geometry/SK_banner01.SK_banner01" true :!label _label))
    (:`Simple Banner`
      (goto _label))
    (:`Square Banner`
      (if (> _type_material_banner 4)
        (set `self.Type Material Banner` 4))
      (`SkinnedMeshComponent.SetSkinnedAssetAndUpdate` _skeletalmesh_2 "/Game/ProceduralBuildings/Geometry/SK_banner02.SK_banner02" true)
      ;[1 0 0] Material
      (set `self.Index Material Banner Offset` 10))
    (:`Flag`
      (if (> _type_material_banner 2)
        (set `self.Type Material Banner` 2))
      (`SkinnedMeshComponent.SetSkinnedAssetAndUpdate` _skeletalmesh_2 "/Game/ProceduralBuildings/Geometry/SK_flag.SK_flag" true)
      (set `self.Index Material Banner Offset` 8)))
  (`PrimitiveComponent.SetMaterial` _skeletalmesh (`MeshComponent.GetMaterialIndex` _skeletalmesh "banner") (`|GetArrayItem` (`self.Materials`) (- (+ (`self.Index Material Banner Offset`) (`self.Type Material Banner`)) 1))))