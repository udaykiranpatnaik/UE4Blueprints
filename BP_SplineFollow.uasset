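; Blueprint actor that spawns static mesh actors evenly spaced along its spline and moves them along it during play.
; BeginPlay spawns one movable actor per MeshList entry and records its start distance, though all receive the list's last mesh.
; The Alpha timeline advances a shared distance, wrapped by spline length, setting each actor's location and rotation plus a local sideways offset.
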(event `self.ReceiveBeginPlay`
  (bind _spline (`self.Spline`))
  ;[1 1 1] Set Up  Actors on Spline
  (set `self.ReadyForAction` false)
  (for (_array_element _array_index) (`self.MeshList`)
    (set `self.CurrentMesh` _array_element)
    (bind _returnvalue (* _array_index (/ (`SplineComponent.GetSplineLength` (`self.Spline`)) (`KismetMathLibrary.Conv_IntToDouble` (`KismetArrayLibrary.Array_Length` (`self.MeshList`))))))
    (`KismetArrayLibrary.Array_Add` (`self.Start`) _returnvalue)
    (bind _returnvalue_2 (`SplineComponent.GetLocationAtDistanceAlongSpline` _spline _returnvalue "World"))
    (`KismetArrayLibrary.Array_Add` (`self.StartPositions`) _returnvalue_2)
    (bind _returnvalue_3 (`|SpawnActorFromClass` "/Script/Engine.StaticMeshActor" (`KismetMathLibrary.MakeTransform` _returnvalue_2 (`SplineComponent.GetRotationAtDistanceAlongSpline` _spline _returnvalue "World")) "Undefined" "OverrideRootScale" null null))
    (`KismetArrayLibrary.Array_Add` (`self.ActorList`) _returnvalue_3))
  (for _array_element_2 (`self.ActorList`)
    (`StaticMeshComponent.SetStaticMesh` (`StaticMeshActor.StaticMeshComponent` _array_element_2) (`self.CurrentMesh`))
    (`StaticMeshActor.SetMobility` _array_element_2 "Movable")
    (bind _output_get (set `self.ReadyForAction` true))
    (if _output_get
      (`self.Animate`))))

(event `SetUp`
  ;[1 1 1] Set Up  Actors on Spline
)

(event `Animate`
  (bind _returnvalue (`SplineComponent.GetSplineLength` (`self.Spline`)))
  (bind (_direction _progress) (`Timeline|Alpha`)
    (:`Update`
      (set `self.SplineCovered` (`KismetMathLibrary.Lerp` 0.0 _returnvalue _progress))
      (for (_array_element _array_index) (`self.ActorList`)
        (bind (_returnvalue_location _returnvalue_rotation) (`KismetMathLibrary.BreakTransform` (`SplineComponent.GetTransformAtDistanceAlongSpline` (`self.Spline`) (mod (+ (`|GetArrayItem` (`self.Start`) _array_index) (`self.SplineCovered`)) _returnvalue) "World" false)))
        (`self.K2_SetActorLocationAndRotation` _array_element _returnvalue_location _returnvalue_rotation false false)
        (`self.K2_AddActorLocalOffset` _array_element (`KismetMathLibrary.MakeVector` 0.0 (`self.SideOffset`)) false false)))))

(fn `UserConstructionScript`)